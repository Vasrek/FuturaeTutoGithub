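; BP_MinionsRanged is a ranged minion character that makes a hitscan attack on a given enemy.
; The StartShooting event line traces on the Visibility channel from the minion to the target's location.
; It applies fixed damage with its controller as instigator only when the first hit is that target, so obstructions block the shot.
; Debug trace drawing and a print on successful hits are left in.
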(event Custom|StartShooting
  (params (EnemyToShoot :type Actor%20Object%20Reference))
  (bind (_outhit _returnvalue) (Collision|LineTraceByChannel (Transformation|GetActorLocation) (Transformation|GetActorLocation EnemyToShoot) "TraceTypeQuery1" false 0 "ForDuration"))
  (if _returnvalue
    (if (== (.HitActor (Collision|BreakHitResult _outhit)) EnemyToShoot)
      (Game|Damage|ApplyDamage (.HitActor (Collision|BreakHitResult _outhit)) 2e+01 (Pawn|GetController) self "/Script/Engine.DamageType")
      (Development|PrintString "Hello"))))

(fn ConstructionScript)